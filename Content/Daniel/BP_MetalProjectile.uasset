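; BP_MetalProjectile is a projectile actor that moves itself along the forward vector of its Sphere component.
; A looping 0.01-second timer started on BeginPlay offsets the actor by MovementDirection and MovementSpeed each tick of the timer, without sweeping or frame-time scaling.
; The Sphere's overlap event checks for the player pawn but takes no action, and a DestroyActor call sits unconnected.
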(event OnComponentBeginOverlap(Sphere)
  (params (OverlappedComponent :type Primitive%20Component%20Object%20Reference) (OtherActor :type Actor%20Object%20Reference) (OtherComp :type Primitive%20Component%20Object%20Reference) (OtherBodyIndex :type Integer) (bFromSweep :type Boolean) (SweepResult :type Hit%20Result%20Structure%20%28by%20ref%29))
  (if (== OtherActor (Game|Player|GetPlayerPawn 0))
    _))

(event Custom|Movement
  (bind _sphere (Variables|Default|GetSphere))
  (Transformation|SetActorLocation (+ (Transformation|GetWorldLocation _sphere) (* (Math|Vector|GetForwardVector _sphere) (Variables|Default|GetMovementDirection) (Variables|Default|GetMovementSpeed))) false false))

(event EventBeginPlay
  (Utilities|Time|SetTimerbyEvent (delegate Custom|Movement) 0.01 true))

(fn ConstructionScript)