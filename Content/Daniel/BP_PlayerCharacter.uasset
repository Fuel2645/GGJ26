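; Player character for a 2D sprite game with side-to-side movement, jump, dash, melee attack and mask-based abilities.
; Enhanced Input drives the actions, with dash launching along the movement direction while friction and gravity are briefly zeroed.
; SelectMask sets which ability fires: Blank and Ink run melee line traces, while Metal spawns a projectile.
; Trace hits and mask animation are print-string placeholders, and the mask selection widget is created but not displayed here.
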(event Input|EnhancedActionEvents|EnhancedInputActionIA_Movement
  (params (ActionValue :type Float%20%28double-precision%29) (ElapsedSeconds :type Float%20%28double-precision%29) (TriggeredSeconds :type Float%20%28double-precision%29) (InputAction :type Input%20Action%20Object%20Reference :default "/Game/Daniel/Input/IA_Movement.IA_Movement"))
  (:Triggered
    (Variables|Movement|SetMovementDirection ActionValue)
    (Pawn|Input|AddMovementInput (Math|Vector|MakeVector ActionValue 0.0 0.0) (Variables|Movement|GetMovementSpeed) false))
  (:Started
    (if (< ActionValue 0.0)
      (Variables|Combat|SetisLeft true)
      (else
        (Variables|Combat|SetisLeft false)))))

(event Input|EnhancedActionEvents|EnhancedInputActionIA_Jump
  (params (ActionValue :type Boolean) (ElapsedSeconds :type Float%20%28double-precision%29) (TriggeredSeconds :type Float%20%28double-precision%29) (InputAction :type Input%20Action%20Object%20Reference :default "/Game/Daniel/Input/IA_Jump.IA_Jump"))
  (:Started
    (if (Pawn|Components|CharacterMovement|IsWalking (Variables|Character|GetCharacterMovement))
      (Character|Jump))))

(event Input|EnhancedActionEvents|EnhancedInputActionIA_Dash
  (params (ActionValue :type Boolean) (ElapsedSeconds :type Float%20%28double-precision%29) (TriggeredSeconds :type Float%20%28double-precision%29) (InputAction :type Input%20Action%20Object%20Reference :default "/Game/Daniel/Input/IA_Dash.IA_Dash"))
  (bind _charactermovement (Variables|Character|GetCharacterMovement))
  (bind _charactermovement_2 (Variables|Character|GetCharacterMovement))
  (:Started
    (if (not (and (Variables|Movement|GetIsDashing) (> (Variables|Movement|GetDashCount) 0)))
      (Variables|Movement|SetIsDashing true)
      (Math|Integer|DecrementInt (Variables|Movement|GetDashCount)
        (:%20%20
          (Variables|/Script/Engine.CharacterMovementComponent|SetGroundFriction _charactermovement 0.0)
          (Variables|/Script/Engine.CharacterMovementComponent|SetGravityScale _charactermovement 0.0)
          (Character|LaunchCharacter (Math|Vector|MakeVector (* (Variables|Movement|GetMovementDirection) (Variables|Movement|GetDashSpeed)) 0.0 0.0) false false)))))
  (:Completed
    (Utilities|FlowControl|Delay 0.2)
    (Variables|/Script/Engine.CharacterMovementComponent|SetGroundFriction _charactermovement_2 (Variables|Movement|GetdefaultGroundFriction))
    (Variables|/Script/Engine.CharacterMovementComponent|SetGravityScale _charactermovement_2 (Variables|Movement|GetdefaultGravity))
    (Utilities|FlowControl|Delay 0.3)
    (Variables|Movement|SetIsDashing false)))

(event Input|EnhancedActionEvents|EnhancedInputActionIA_Attack
  (params (ActionValue :type Boolean) (ElapsedSeconds :type Float%20%28double-precision%29) (TriggeredSeconds :type Float%20%28double-precision%29) (InputAction :type Input%20Action%20Object%20Reference :default "/Game/Daniel/Input/IA_Attack.IA_Attack"))
  (bind _papersprite (Variables|Default|GetPaperSprite))
  (bind _returnvalue (Transformation|GetWorldLocation _papersprite))
  (:Started
    (if (not (Variables|Combat|GetisAttacking))
      (Collision|MultiLineTraceByChannel _returnvalue (+ _returnvalue (* (Math|Vector|GetForwardVector _papersprite) (Variables|Combat|GetMeleeDistance) (Variables|Movement|GetMovementDirection))) "TraceTypeQuery1" false 0 "ForDuration")
      (Development|PrintString "Call Hits")
      (Variables|Combat|SetisAttacking true)))
  (:Completed
    (Utilities|FlowControl|Delay 0.3)
    (Variables|Combat|SetisAttacking false)))

(event Input|EnhancedActionEvents|EnhancedInputActionIA_Ability
  (params (ActionValue :type Boolean) (ElapsedSeconds :type Float%20%28double-precision%29) (TriggeredSeconds :type Float%20%28double-precision%29) (InputAction :type Input%20Action%20Object%20Reference :default "/Game/Daniel/Input/IA_Ability.IA_Ability"))
  (:Started
    (if (not (Variables|Combat|GetisAttacking))
      (Variables|Combat|SetisAttacking false)
      (switch Utilities|FlowControl|Switch|SwitchonEMaskTypes (Variables|Combat|GetSelected%20Mask)
        (:NewEnumerator0
          (CallFunction|BlankAbility))
        (:NewEnumerator2
          (CallFunction|InkAbility))
        (:NewEnumerator3
          (CallFunction|MetalAbility)))))
  (:Completed
    (Utilities|FlowControl|Delay 0.3)
    (Variables|Combat|SetisAttacking false)))

(event EventBeginPlay
  (bind _charactermovement (Variables|Character|GetCharacterMovement))
  (Input|AddMappingContext (PlayerController|LocalPlayerSubsystems|GetEnhancedInputLocalPlayerSubsystem (Game|GetPlayerController 0)) "/Game/Daniel/Input/IMC_Player.IMC_Player" 0 "(bIgnoreAllPressedKeysUntilRelease=True,bForceImmediately=False,bNotifyUserSettings=False)")
  (Variables|Movement|SetdefaultGroundFriction (Variables|/Script/Engine.CharacterMovementComponent|GetGroundFriction _charactermovement))
  (Variables|Movement|SetdefaultGravity (Variables|/Script/Engine.CharacterMovementComponent|GetGravityScale _charactermovement))
  (bind _returnvalue (UserInterface|CreateWidget "/Game/Daniel/Widget/WBP_MaskSelect.WBP_MaskSelect_C"))
  (Variables|Widget|SetmaskSelection%20Widget _returnvalue))

(event EventSelectMask
  (params (New%20Mask :type EMaskTypes%20Enum :default "NewEnumerator0"))
  (bind _output_get (Variables|Combat|SetSelected%20Mask New%20Mask))
  (Development|PrintString "Play Animation")
  (Development|PrintString (Utilities|String|EnumtoString _output_get)))

(fn ConstructionScript)

(fn BlankAbility
  (bind _papersprite (Variables|Default|GetPaperSprite))
  (bind _returnvalue (Transformation|GetWorldLocation _papersprite))
  (Collision|MultiLineTraceByChannel _returnvalue (+ _returnvalue (* (Math|Vector|GetForwardVector _papersprite) (Variables|Combat|GetMeleeDistance) (Variables|Movement|GetMovementDirection))) "TraceTypeQuery1" false 0 "ForDuration")
  (Development|PrintString "Call Hits")
  (Variables|Combat|SetisAttacking true))

(fn InkAbility
  (bind _papersprite (Variables|Default|GetPaperSprite))
  (bind _returnvalue (Transformation|GetWorldLocation _papersprite))
  (Collision|MultiLineTraceByChannel _returnvalue (+ _returnvalue (* (Math|Vector|GetForwardVector _papersprite) (Variables|Combat|GetMeleeDistance) (Variables|Movement|GetMovementDirection))) "TraceTypeQuery1" false 0 "ForDuration")
  (Development|PrintString "Call Hits 
Call DotS 
")
  (Variables|Combat|SetisAttacking true))

(fn MetalAbility
  (bind _papersprite (Variables|Default|GetPaperSprite))
  (bind _returnvalue (Game|SpawnActorfromClass "/Game/Daniel/BP_MetalProjectile.BP_MetalProjectile_C" (Math|Transform|MakeTransform (+ (Transformation|GetWorldLocation _papersprite) (* (Math|Vector|GetForwardVector _papersprite) (* (Variables|Movement|GetMovementDirection) 5e+01))) "0, 0, 0" "1.000000,1.000000,1.000000") "Undefined" "MultiplyWithRoot" 0 0))
  (Variables|/Game/Daniel/BP_MetalProjectile.BP_MetalProjectile_C|SetMovementDirection _returnvalue (Variables|Movement|GetMovementDirection)))