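; Player character for a 2D side-scroller with movement, jump, gravity-free dash, melee attack and mask-based abilities.
; The selected mask picks a cooldown-gated ability: Blank heavy hit, Ink damage-over-time hit or Metal projectile.
; Melee hits use forward line traces, with debug drawing, that message actors implementing BPI_EnemyInteraction.
; BeginPlay teleports to the current checkpoint; zero HP pauses into a death screen, and T is a debug kill.
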(event Input|EnhancedActionEvents|EnhancedInputActionIA_Movement
  (params (ActionValue :type Float%20%28double-precision%29) (ElapsedSeconds :type Float%20%28double-precision%29) (TriggeredSeconds :type Float%20%28double-precision%29) (InputAction :type Input%20Action%20Object%20Reference :default "/Game/Daniel/Input/IA_Movement.IA_Movement"))
  (:Triggered
    (Variables|Movement|SetMovementDirection ActionValue)
    (Pawn|Input|AddMovementInput (Math|Vector|MakeVector ActionValue 0.0 0.0) (Variables|Movement|GetMovementSpeed) false))
  (:Started
    (if (< ActionValue 0.0)
      (Variables|Combat|SetisLeft true)
      (else
        (Variables|Combat|SetisLeft false)))))

(event Input|EnhancedActionEvents|EnhancedInputActionIA_Jump
  (params (ActionValue :type Boolean) (ElapsedSeconds :type Float%20%28double-precision%29) (TriggeredSeconds :type Float%20%28double-precision%29) (InputAction :type Input%20Action%20Object%20Reference :default "/Game/Daniel/Input/IA_Jump.IA_Jump"))
  (:Started
    (if (Pawn|Components|CharacterMovement|IsWalking (Variables|Character|GetCharacterMovement))
      (Character|Jump))))

(event Input|EnhancedActionEvents|EnhancedInputActionIA_Dash
  (params (ActionValue :type Boolean) (ElapsedSeconds :type Float%20%28double-precision%29) (TriggeredSeconds :type Float%20%28double-precision%29) (InputAction :type Input%20Action%20Object%20Reference :default "/Game/Daniel/Input/IA_Dash.IA_Dash"))
  (bind _charactermovement (Variables|Character|GetCharacterMovement))
  (bind _charactermovement_2 (Variables|Character|GetCharacterMovement))
  (:Started
    (if (not (and (Variables|Movement|GetIsDashing) (> (Variables|Movement|GetDashCount) 0)))
      (Variables|Movement|SetIsDashing true)
      (Math|Integer|DecrementInt (Variables|Movement|GetDashCount)
        (:%20%20
          (Variables|/Script/Engine.CharacterMovementComponent|SetGroundFriction _charactermovement 0.0)
          (Variables|/Script/Engine.CharacterMovementComponent|SetGravityScale _charactermovement 0.0)
          (Character|LaunchCharacter (Math|Vector|MakeVector (* (Variables|Movement|GetMovementDirection) (Variables|Movement|GetDashSpeed)) 0.0 0.0) false false)))))
  (:Completed
    (Utilities|FlowControl|Delay 0.2)
    (Variables|/Script/Engine.CharacterMovementComponent|SetGroundFriction _charactermovement_2 (Variables|Movement|GetdefaultGroundFriction))
    (Variables|/Script/Engine.CharacterMovementComponent|SetGravityScale _charactermovement_2 (Variables|Movement|GetdefaultGravity))
    (Utilities|FlowControl|Delay 0.3)
    (Variables|Movement|SetIsDashing false)))

(event Input|EnhancedActionEvents|EnhancedInputActionIA_Attack
  (params (ActionValue :type Boolean) (ElapsedSeconds :type Float%20%28double-precision%29) (TriggeredSeconds :type Float%20%28double-precision%29) (InputAction :type Input%20Action%20Object%20Reference :default "/Game/Daniel/Input/IA_Attack.IA_Attack"))
  (bind _papersprite (Variables|Default|GetPaperSprite))
  (bind _returnvalue (Transformation|GetWorldLocation _papersprite))
  (:Started
    (if (not (Variables|Combat|GetisAttacking))
      (bind _outhits (Collision|MultiLineTraceByChannel _returnvalue (+ _returnvalue (* (Math|Vector|GetForwardVector _papersprite) (Variables|Combat|GetMeleeDistance) (Variables|Movement|GetMovementDirection))) "TraceTypeQuery1" false 0 "ForDuration"))
      (for _array_element _outhits
        (if (Utilities|DoesObjectImplementInterface (.HitActor (Collision|BreakHitResult _array_element)) "/Game/Daniel/Interfaces/BPI_EnemyInteraction.BPI_EnemyInteraction_C")
          (Class|BPIEnemyInteraction|Damage(Message) (.HitActor (Collision|BreakHitResult _array_element)) 3e+01)))
      (Variables|Combat|SetisAttacking true)))
  (:Completed
    (Utilities|FlowControl|Delay 0.3)
    (Variables|Combat|SetisAttacking false)))

(event Input|EnhancedActionEvents|EnhancedInputActionIA_Ability
  (params (ActionValue :type Boolean) (ElapsedSeconds :type Float%20%28double-precision%29) (TriggeredSeconds :type Float%20%28double-precision%29) (InputAction :type Input%20Action%20Object%20Reference :default "/Game/Daniel/Input/IA_Ability.IA_Ability"))
  (:Started
    (if (not (Variables|Combat|GetisAttacking))
      (Variables|Combat|SetisAttacking false)
      (switch Utilities|FlowControl|Switch|SwitchonEMaskTypes (Variables|Combat|GetSelected%20Mask)
        (:NewEnumerator0
          (if (Variables|Cooldowns|GetisBlankReady)
            (CallFunction|BlankAbility)
            (Variables|Cooldowns|SetisBlankReady false)
            (Utilities|FlowControl|Delay (Variables|Cooldowns|GetBlank%20Ability%20Cooldown))
            (Variables|Cooldowns|SetisBlankReady true)))
        (:NewEnumerator2
          (if (Variables|Cooldowns|GetisInkReady)
            (CallFunction|InkAbility)
            (Variables|Cooldowns|SetisInkReady false)
            (Utilities|FlowControl|Delay (Variables|Cooldowns|GetInk%20Ability%20Cooldown))
            (Variables|Cooldowns|SetisInkReady true)))
        (:NewEnumerator3
          (if (Variables|Cooldowns|GetisMetalReady)
            (CallFunction|MetalAbility)
            (Variables|Cooldowns|SetisMetalReady false)
            (Utilities|FlowControl|Delay (Variables|Cooldowns|GetMetal%20Ability%20Cooldown))
            (Variables|Cooldowns|SetisMetalReady true))))))
  (:Completed
    (Utilities|FlowControl|Delay 0.3)
    (Variables|Combat|SetisAttacking false)))

(event EventBeginPlay
  (bind _charactermovement (Variables|Character|GetCharacterMovement))
  (Input|AddMappingContext (PlayerController|LocalPlayerSubsystems|GetEnhancedInputLocalPlayerSubsystem (Game|GetPlayerController 0)) "/Game/Daniel/Input/IMC_Player.IMC_Player" 0 "(bIgnoreAllPressedKeysUntilRelease=True,bForceImmediately=False,bNotifyUserSettings=False)")
  (Variables|Movement|SetdefaultGroundFriction (Variables|/Script/Engine.CharacterMovementComponent|GetGroundFriction _charactermovement))
  (Variables|Movement|SetdefaultGravity (Variables|/Script/Engine.CharacterMovementComponent|GetGravityScale _charactermovement))
  (bind _returnvalue (UserInterface|CreateWidget "/Game/Daniel/Widget/WBP_MaskSelect.WBP_MaskSelect_C"))
  (Variables|Widget|SetmaskSelection%20Widget _returnvalue)
  (CallFunction|Initalise))

(event EventSelectMask
  (params (New%20Mask :type EMaskTypes%20Enum :default "NewEnumerator0"))
  (bind _output_get (Variables|Combat|SetSelected%20Mask New%20Mask))
  (Development|PrintString "Play Animation")
  (Development|PrintString (Utilities|String|EnumtoString _output_get)))

(event EventDamage
  (params (dam :type Float%20%28double-precision%29))
  (bind _output_get (Variables|Default|SetHP (Math|Float|Clamp(Float) (- (Variables|Default|GetHP) dam) 0.0 (Variables|Default|GetMaxHP))))
  (if (<= _output_get 0.0)
    (Game|SetGamePaused true)
    (bind _returnvalue (UserInterface|CreateWidget "/Game/Daniel/Widget/WBP_DeathScreen.WBP_DeathScreen_C"))
    (Input|SetInputModeUIOnly (Game|GetPlayerController 0) _returnvalue "DoNotLock" true)
    (UserInterface|Viewport|AddtoViewport _returnvalue 0)
    (Variables|/Script/Engine.PlayerController|SetbShowMouseCursor (Game|GetPlayerController 0) true)))

(event EventInitalise
  (Variables|Default|SetHP 1e+02)
  (Variables|Default|SetMaxHP 1e+02)
  (bind _outactors (Actor|GetAllActorsOfClass "/Game/Daniel/Blueprints/BP_Checkpoint.BP_Checkpoint_C"))
  (for _array_element _outactors
    (if (== (Variables|/Game/Daniel/Blueprints/BP_Checkpoint.BP_Checkpoint_C|GetCheckPoint%20Num _array_element) (Variables|Default|GetCurrentCheckpoint))
      (Transformation|SetActorLocation (Transformation|GetActorLocation _array_element) false true))))

(event EventCheckpointReached
  (params (Checkpoint%20Num :type Integer))
  (if (not (<= Checkpoint%20Num (Variables|Default|GetCurrentCheckpoint)))
    (Variables|Default|SetCurrentCheckpoint Checkpoint%20Num)))

(event Input|KeyboardEvents|T
  (params (Key :type Key%20Structure :default "None"))
  (:Pressed
    (CallFunction|Damage 1e+02 :!label _label))
  (:Released
    (goto _label)))

(fn ConstructionScript)

(fn BlankAbility
  (bind _papersprite (Variables|Default|GetPaperSprite))
  (bind _returnvalue (Transformation|GetWorldLocation _papersprite))
  (bind _outhits (Collision|MultiLineTraceByChannel _returnvalue (+ _returnvalue (* (Math|Vector|GetForwardVector _papersprite) (Variables|Combat|GetMeleeDistance) (Variables|Movement|GetMovementDirection))) "TraceTypeQuery1" false 0 "ForDuration"))
  (for _array_element _outhits
    (if (Utilities|DoesObjectImplementInterface (.HitActor (Collision|BreakHitResult _array_element)) "/Game/Daniel/Interfaces/BPI_EnemyInteraction.BPI_EnemyInteraction_C")
      (Class|BPIEnemyInteraction|Damage(Message) (.HitActor (Collision|BreakHitResult _array_element)) 5e+01)))
  (Variables|Combat|SetisAttacking true))

(fn InkAbility
  (bind _papersprite (Variables|Default|GetPaperSprite))
  (bind _returnvalue (Transformation|GetWorldLocation _papersprite))
  (bind _outhits (Collision|MultiLineTraceByChannel _returnvalue (+ _returnvalue (* (Math|Vector|GetForwardVector _papersprite) (Variables|Combat|GetMeleeDistance) (Variables|Movement|GetMovementDirection))) "TraceTypeQuery1" false 0 "ForDuration"))
  (for _array_element _outhits
    (if (Utilities|DoesObjectImplementInterface (.HitActor (Collision|BreakHitResult _array_element)) "/Game/Daniel/Interfaces/BPI_EnemyInteraction.BPI_EnemyInteraction_C")
      (Class|BPIEnemyInteraction|InkDamage(Message) (.HitActor (Collision|BreakHitResult _array_element)) 2e+01 5.0 0.5 5)))
  (Variables|Combat|SetisAttacking true))

(fn MetalAbility
  (bind _papersprite (Variables|Default|GetPaperSprite))
  (bind _returnvalue (Game|SpawnActorfromClass "/Game/Daniel/Blueprints/BP_MetalProjectile.BP_MetalProjectile_C" (Math|Transform|MakeTransform (+ (Transformation|GetWorldLocation _papersprite) (* (Math|Vector|GetForwardVector _papersprite) (* (Variables|Movement|GetMovementDirection) 5e+01))) "0, 0, 0" "1.000000,1.000000,1.000000") "Undefined" "MultiplyWithRoot" 0 0))
  (Variables|/Game/Daniel/Blueprints/BP_MetalProjectile.BP_MetalProjectile_C|SetMovementDirection _returnvalue (Variables|Movement|GetMovementDirection)))