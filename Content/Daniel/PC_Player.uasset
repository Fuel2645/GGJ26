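; PC_Player is a player controller that shows a mask selection widget while the mask select input is held.
; It creates a WBP_MaskSelect widget once at BeginPlay and stores it for reuse.
; Enhanced Input IA_MaskSelect adds the widget to the viewport and centers the mouse on Started, then removes it on Completed.
; The MaskSelectionCheck function is an empty stub.
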(event Input|EnhancedActionEvents|EnhancedInputActionIA_MaskSelect
  (params (ActionValue :type Boolean) (ElapsedSeconds :type Float%20%28double-precision%29) (TriggeredSeconds :type Float%20%28double-precision%29) (InputAction :type Input%20Action%20Object%20Reference :default "/Game/Daniel/Input/IA_MaskSelect.IA_MaskSelect"))
  (bind _returnvalue (Viewport|GetViewportSize))
  (bind _maskselection_widget (Variables|Default|GetmaskSelection%20Widget))
  (bind _returnvalue_2 (/ _returnvalue 2.0))
  (:Started
    (UserInterface|Viewport|AddtoViewport _maskselection_widget 0)
    (Class|PlayerController|SetMouseLocation (Math|Float|Truncate (.x _returnvalue_2)) (Math|Float|Truncate (.y _returnvalue_2))))
  (:Completed
    (Widget|RemovefromParent _maskselection_widget)))

(event EventBeginPlay
  (bind _returnvalue (UserInterface|CreateWidget "/Game/Daniel/Widget/WBP_MaskSelect.WBP_MaskSelect_C"))
  (Variables|Default|SetmaskSelection%20Widget _returnvalue))

(fn ConstructionScript)

(fn MaskSelectionCheck)