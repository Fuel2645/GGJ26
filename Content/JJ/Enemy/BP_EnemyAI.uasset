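; BP_EnemyAI is an enemy actor that patrols back and forth along a spline path.
; Each Tick advances a distance by EnemySpeed and delta time, then sets the Enemy component's relative location and rotation from the spline's local transform.
; Reaching either end sets a hardcoded positive or negative speed to reverse travel.
; The IsReversing check always passes because the flag is set true just before it.
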(event EventTick
  (params (DeltaSeconds :type Float%20%28single-precision%29))
  (Variables|Default|SetDistance%20Along%20Spline (+ (* DeltaSeconds (Variables|Default|GetEnemy%20Speed)) (Variables|Default|GetDistance%20Along%20Spline)))
  (Transformation|SetRelativeTransform (Variables|Default|GetEnemy) (Math|Transform|MakeTransform (.location (Spline|GetTransformatDistanceAlongSpline (Variables|Default|GetSpline) (Variables|Default|GetDistance%20Along%20Spline) "Local" false)) (.rotation (Spline|GetTransformatDistanceAlongSpline (Variables|Default|GetSpline) (Variables|Default|GetDistance%20Along%20Spline) "Local" false)) "1.000000,1.000000,1.000000") false false)
  (Variables|Default|SetIsReversing true)
  (if (Variables|Default|GetIsReversing)
    (if (>= (Variables|Default|GetDistance%20Along%20Spline) (Spline|GetSplineLength (Variables|Default|GetSpline)))
      (Variables|Default|SetEnemy%20Speed -2.5e+02)
      (elif (<= (Variables|Default|GetDistance%20Along%20Spline) 0.0)
        (Variables|Default|SetEnemy%20Speed 2.5e+02)
        (Variables|Default|SetIsReversing false)))))

(fn ConstructionScript)